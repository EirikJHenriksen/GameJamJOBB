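; BP_Worker is an actor representing a worker who is either working or slacking, shown by the material on its Workerbox component.
; On BeginPlay it randomly picks the IsWorking state and calls UpdateLook to apply the matching material.
; YelledAt sets a slacker to working and updates its look, printing a green Norwegian reply, while an already working worker just prints a red frown.
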(event `self.ReceiveBeginPlay`
  (set `self.IsWorking` (`KismetMathLibrary.Conv_IntToBool` (`KismetMathLibrary.RandomIntegerInRange` 0 1)))
  (`self.UpdateLook`))

(fn `UpdateLook`
  (bind _workerbox (`self.Workerbox`))
  (if (`self.IsWorking`)
    (`PrimitiveComponent.SetMaterial` _workerbox 0 (`self.MaterialWorking`))
    (else
      (`PrimitiveComponent.SetMaterial` _workerbox 0 (`self.MaterialSlacking`)))))

(fn `UserConstructionScript`)

(fn `YelledAt`
  (if (`self.IsWorking`)
    (`KismetSystemLibrary.PrintString` ":(" true true (struct :`R` 1.0 :`G` 0.026519 :`A` 1.0))
    (else
      (set `self.IsWorking` true)
      (`self.UpdateLook`)
      (`KismetSystemLibrary.PrintString` "(O.o) \"Den er grei, sjef!\"" true true (struct :`R` 0.118336 :`G` 1.0 :`A` 1.0)))))